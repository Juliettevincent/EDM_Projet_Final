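; BP_CLOCK is a Blueprint that runs a Quartz musical clock and displays its beat position for debugging.
; On BeginPlay it creates "MainClock" through the Quartz subsystem, sets its tempo from BeatsPerMinute and starts it.
; It then subscribes to quarter-note quantization events, with a handler that prints the clock name, bar and beat under a fixed message key.
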(event Custom|CustomEvent
  (params (ClockName :type Name) (QuantizationType :type EQuartzCommandQuantization%20Enum :default "Bar") (NumBars :type Integer) (Beat :type Integer) (BeatFraction :type Float%20%28single-precision%29))
  (Development|PrintString (Utilities|String|ToString(Text) (Utilities|Text|FormatText "{clock} {bar} {beat}" ClockName NumBars Beat)) true true "(R=0.000000,G=0.660000,B=1.000000,A=1.000000)" 2.0 "Clock"))

(event EventBeginPlay
  (bind _returnvalue (Class|QuartzSubsystem|CreateNewClock :self (WorldSubsystems|GetQuartzSubsystem) :ClockName "MainClock"))
  ;[0.15 0.15 0.15 0.5] Comment
  (bind _output_get (Variables|Default|SetMainClock _returnvalue))
  ;[0.15 0.15 0.15 0.5] Configurer le BPM
  (bind _clockhandle (Class|QuartzClockHandle|SetBeatsPerMinute :self _output_get :BeatsPerMinute (Variables|Default|GetBeats%20Per%20Minute)))
  ;[0.15 0.15 0.15 0.5] Demarrer
  (bind _clockhandle_2 (Class|QuartzClockHandle|StartClock _clockhandle))
  (Class|QuartzClockHandle|SubscribetoQuantizationEvent _clockhandle_2 "QuarterNote" (EventDispatchers|CreateEvent :!event Custom|CustomEvent)))

(fn ConstructionScript)